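; BP_Button is a VR button that starts the game when the BP_MyVRPawn overlaps its mesh.
; A timeline scales the mesh; finishing forward plays a sound, then calls StartGame on BP_MyVRGamemode after a short delay.
; Touches during play only trigger the sound.
; The game mode's candy-removal event, bound on BeginPlay, reverses the timeline to reset the button.
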(event OnComponentBeginOverlap(ButtonMesh)
  (params (OverlappedComponent :type Primitive%20Component%20Object%20Reference) (OtherActor :type Actor%20Object%20Reference) (OtherComp :type Primitive%20Component%20Object%20Reference) (OtherBodyIndex :type Integer) (bFromSweep :type Boolean) (SweepResult :type Hit%20Result%20Structure%20%28by%20ref%29))
  (bind _returnvalue (Transformation|GetActorLocation))
  ;[1 1 1] Button press animation and game start
  (bind _asbp_my_vrgamemode (Utilities|Casting|CastToBP_MyVRGamemode (Game|GetGameMode)))
  (if (== (Utilities|GetClass OtherActor) "/Game/Assets/player/bp_MyVRPawn.BP_MyVRPawn_C")
    (if (Variables|/Game/Assets/player/BP_MyVRGamemode.BP_MyVRGamemode_C|GetisPlaying _asbp_my_vrgamemode)
      (Audio|PlaySoundatLocation "/Game/Assets/audio/button_Cue.button_Cue" _returnvalue)
      (else
        (bind (_direction _alpha) (Timeline|Animation Play)
          (:Update
            (Transformation|SetRelativeScale3D (Variables|Default|GetButtonMesh) (Math|Vector|Lerp(Vector) (Variables|Default|GetstartingScale) (Variables|Default|GetendingScale) _alpha)))
          (:Finished
            (if (Utilities|Enum|Equal(Enum) _direction "Forward")
              (Audio|PlaySoundatLocation "/Game/Assets/audio/button_Cue.button_Cue" _returnvalue)
              (Utilities|FlowControl|Delay 2.0)
              (Default|StartGame _asbp_my_vrgamemode))))))))

(event Custom|RestButton
  ;[1 1 1] Button press animation and game start
  (bind (_direction _alpha) (Timeline|Animation Reverse)
    (:Update
      (Transformation|SetRelativeScale3D (Variables|Default|GetButtonMesh) (Math|Vector|Lerp(Vector) (Variables|Default|GetstartingScale) (Variables|Default|GetendingScale) _alpha)))
    (:Finished
      (if (Utilities|Enum|Equal(Enum) _direction "Forward")
        (Audio|PlaySoundatLocation "/Game/Assets/audio/button_Cue.button_Cue" (Transformation|GetActorLocation))
        (Utilities|FlowControl|Delay 2.0)
        (Default|StartGame (stale OnComponentBeginOverlap(ButtonMesh) _asbp_my_vrgamemode))))))

(event EventBeginPlay
  ;[1 1 1] Bind to candies remove
  (bind _asbp_my_vrgamemode (Utilities|Casting|CastToBP_MyVRGamemode (Game|GetGameMode)))
  (bind _output_get (Variables|Default|SetmyVRGameMode _asbp_my_vrgamemode))
  (EventDispatchers|BindEventtoRemoveCandy _output_get (delegate Custom|RestButton)))

(event Collision|EventActorBeginOverlap
  (params (OtherActor :type Actor%20Object%20Reference)))

(event EventTick
  (params (DeltaSeconds :type Float%20%28single-precision%29)))

(fn ConstructionScript)