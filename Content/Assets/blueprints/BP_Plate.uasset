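; BP_Plate is a plate actor in a VR candy game that scores candy placed on it.
; On actor overlap with a BP_Candy, it sets the candy's IsCandyOnPlate flag to prevent repeat counting and plays an eating sound at the plate mesh.
; It then has BP_MyVRGamemode increase the score, destroys the candy immediately despite first setting a lifespan, and asks the game mode to spawn another candy.
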(event EventBeginPlay)

(event Collision|EventActorBeginOverlap
  (params (OtherActor :type Actor%20Object%20Reference))
  ;[1 1 1] Put candy on plate and increase score
  (Utilities|IsValid OtherActor
    (:Is%20Valid
      (bind _asbp_candy (Utilities|Casting|CastToBP_Candy OtherActor))
      (if (not (Variables|/Game/Assets/blueprints/BP_Candy.BP_Candy_C|GetisCandyOnPlate _asbp_candy))
        (Variables|/Game/Assets/blueprints/BP_Candy.BP_Candy_C|SetisCandyOnPlate _asbp_candy true)
        (Audio|PlaySoundatLocation "/Game/Assets/audio/eat_candy_Cue.eat_candy_Cue" (Transformation|GetWorldLocation (Variables|Default|GetPlateMesh)))
        (Actor|SetLifeSpan _asbp_candy 1.0)
        (bind _asbp_my_vrgamemode (Utilities|Casting|CastToBP_MyVRGamemode (Game|GetGameMode)))
        (Default|IncreaseScore _asbp_my_vrgamemode)
        (Actor|DestroyActor _asbp_candy)
        (Default|SpawnCandy _asbp_my_vrgamemode)))))

(event EventTick
  (params (DeltaSeconds :type Float%20%28single-precision%29))
  ;[1 1 1] Put candy on plate and increase score
)

(fn ConstructionScript)