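; BP_Candy is a VR candy actor that can be picked up and dropped.
; PickUp turns off mesh physics and attaches the root to the supplied component, unless the candy is flagged as on a plate.
; DropOff re-enables physics and detaches it, keeping its world transform.
; On BeginPlay it binds to an event on BP_MyVRGamemode that destroys the candy when fired.
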(event Custom|RemoveCandyEvent
  ;[1 1 1] Event to remove candy from game
  (Actor|DestroyActor))

(event EventBeginPlay
  ;[1 1 1] Prepare candy to remove
  (bind _asbp_my_vrgamemode (Utilities|Casting|CastToBP_MyVRGamemode (Game|GetGameMode)))
  (bind _output_get (Variables|Default|SetmyVRGameMode _asbp_my_vrgamemode))
  (EventDispatchers|BindEventtoRemoveCandy _output_get (delegate Custom|RemoveCandyEvent)))

(event Collision|EventActorBeginOverlap
  (params (OtherActor :type Actor%20Object%20Reference)))

(event EventTick
  (params (DeltaSeconds :type Float%20%28single-precision%29)))

(event EventDropOff
  ;[1 1 1] Drop off candy
  (Physics|SetSimulatePhysics (Variables|Default|GetCandyMesh) true)
  (Transformation|DetachFromActor "KeepWorld" "KeepWorld" "KeepWorld"))

(event EventPickUp
  (params (ActorToAttachTo :type Scene%20Component%20Object%20Reference))
  ;[1 1 1] Pick up candy
  (if (not (Variables|Default|GetisCandyOnPlate))
    (Physics|SetSimulatePhysics (Variables|Default|GetCandyMesh) false)
    (Transformation|AttachComponentToComponent (VehicleSound|GetRootComponent) ActorToAttachTo "None" "KeepWorld" "KeepWorld" "KeepWorld" true)))

(fn ConstructionScript)