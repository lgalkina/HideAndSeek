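; VR game mode Blueprint that runs a timed candy game, tracking score, time left and play state.
; StartGame resets score and timer, then spawns a BP_Candy at a random TargetPoint in the level.
; Tick uses a Delay as a one-second countdown; at zero it plays the game-over sound, stops play and calls RemoveCandy.
; IncreaseScore adds one point and returns the new score.
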(event EventBeginPlay)

(event EventTick
  (params (DeltaSeconds :type Float%20%28single-precision%29))
  ;[1 1 1] Game
  (if (Variables|Default|GetisPlaying)
    (Utilities|FlowControl|Delay 1.0)
    (if (Variables|Default|GetisPlaying)
      (Variables|Default|SettimeLeft (- (Variables|Default|GettimeLeft) 1))
      (if (<= (Variables|Default|GettimeLeft) 0)
        (Audio|SpawnSound2D "/Game/Assets/audio/game_over_Cue.game_over_Cue")
        (Variables|Default|SetisPlaying false)
        (Default|CallRemoveCandy)))))

(fn ConstructionScript)

(fn IncreaseScore
  ;[1 1 1] Increase score
  (bind _output_get (Variables|Default|Setscore (+ (Variables|Default|Getscore) 1)))
  (return _output_get))

(fn StartGame
  ;[1 1 1] Set variables to start the game
  (Variables|Default|SetisPlaying true)
  (Variables|Default|Setscore 0)
  (Variables|Default|SettimeLeft 120)
  (CallFunction|SpawnCandy))

(fn SpawnCandy
  ;[1 1 1] Spawn candy in one of predefined target points
  (if (Variables|Default|GetisPlaying)
    (bind _outactors (Actor|GetAllActorsOfClass "/Script/Engine.TargetPoint"))
    (Game|SpawnActorfromClass "/Game/Assets/blueprints/BP_Candy.BP_Candy_C" (Transformation|GetActorTransform (Utilities|Array|Get(acopy) _outactors (Math|Random|RandomIntegerinRange 0 (- (Utilities|Array|Length _outactors) 1)))) "Undefined" 0 0)))